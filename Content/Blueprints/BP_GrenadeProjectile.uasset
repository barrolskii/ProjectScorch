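; Grenade projectile actor that explodes on a roughly one-second fuse, damaging actors around it.
; The fuse is a Delay driven from Tick rather than BeginPlay, leading into the Explode event.
; Explode spawns an explosion particle effect, applies radial damage credited to its instigator, draws a debug sphere matching the damage radius, then destroys the actor.
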(event `self.ReceiveTick`
  (params (DeltaSeconds :type "Float (single-precision)"))
  (`KismetSystemLibrary.Delay` 1.0)
  (`self.Explode`))

(event `Explode`
  (`GameplayStatics.SpawnEmitterAtLocation` "/Game/WeaponEffects/Explosion/P_Explosion.P_Explosion" (`self.K2_GetActorLocation`))
  (`GameplayStatics.ApplyRadialDamage` :`BaseDamage` 40.0 :`Origin` (`self.K2_GetActorLocation`) :`DamageRadius` 200.0 :`DamageCauser` self :`InstigatedByController` (`self.GetInstigatorController`))
  (`KismetSystemLibrary.DrawDebugSphere` (`self.K2_GetActorLocation`) 200.0 12 (struct :`R` 0.173063 :`G` 0.079419 :`B` 1.0 :`A` 1.0) 1.0 3.0)
  (`self.K2_DestroyActor`))

(fn `UserConstructionScript`)